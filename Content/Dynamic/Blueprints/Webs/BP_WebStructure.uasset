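; Player-style web structure actor, built from placed impact points up to a maximum count and turned into a procedural mesh with collision.
; During placement, gravity-free translucent cables preview the links between points, with a sound per shot.
; Ending placement fan-triangulates around the averaged center, adds web-material cables and returns point count as consumption score, or destroys the actor below three points.
; Cleanup removes mesh and cables and plays a destruction sound.
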(event `self.ReceiveDestroyed`
  (`self.ClearIndicators`))

(fn `AddToPlacement`
  (params (ImpactLocation :type "Vector Structure"))
  (returns (ConsumptionScore :type "Float (double-precision)"))
  (bind _webpoints (`self.WebPoints`))
  (if (`self.ReachedMaxWebPoints`)
    (bind _returnvalue (`KismetArrayLibrary.Array_Add` _webpoints ImpactLocation))
    (bind _cable (`self.CreateIndicator` ImpactLocation (`|GetArrayItem` _webpoints (- _returnvalue 1))))
    (`KismetArrayLibrary.Array_Add` (`self.IndicatorCables`) _cable)
    (`GameplayStatics.PlaySoundAtLocation` "/Game/Dynamic/Sound/S_WebStructureShoot.S_WebStructureShoot" ImpactLocation (struct) 1.0 1.0 0.0 null null null null)))

(fn `CleanupWeb`
  (`ActorComponent.K2_DestroyComponent` (`self.ProceduralMesh`))
  (`self.ClearIndicators`)
  (`self.PlayDestructionSound` (`self.Center`)))

(fn `ClearIndicators`
  (for _array_element (`self.IndicatorCables`)
    (`/Engine/EditorBlueprintResources/StandardMacros.IsValid` _array_element
      (:`Is Valid`
        (`ActorComponent.K2_DestroyComponent` _array_element)))))

(fn `CreateIndicator`
  (params (Begin :type "Vector Structure") (End :type "Vector Structure"))
  (returns (Cable :type "CableComponent Object Reference"))
  ;[1 1 1] Create cable basics
  (bind _returnvalue (`AddComponent|NODE_AddCableComponent-0` :`RelativeTransform` (`KismetMathLibrary.MakeTransform` Begin)))
  (`PrimitiveComponent.SetMaterial` _returnvalue 0 "/Game/Static/Material/MI_WebTranslucent.MI_WebTranslucent")
  (set `CableComponent.EndLocation` End _returnvalue)
  (set `CableComponent.CableWidth` (`self.Indicator Width`) _returnvalue)
  ;[1 1 1] Disable physics
  (set `CableComponent.bEnableStiffness` true _returnvalue)
  (set `PrimitiveComponent.bGenerateOverlapEvents` false _returnvalue)
  (set `CableComponent.CableGravityScale` 0.0 _returnvalue)
  (return _returnvalue))

(fn `EndPlacement`
  (params (ImpactLocation :type "Vector Structure"))
  (returns (ConsumptionScore :type "Float (double-precision)"))
  (locals (UVs :type "Array of Vector2D Structure"))
  (bind _webpoints (`self.WebPoints`))
  (bind _uvs (`local.UVs`))
  (bind _proceduralmesh (`self.ProceduralMesh`))
  (bind _webpoints_2 (`self.WebPoints`))
  (bind _webpoints_3 (`self.WebPoints`))
  (bind _returnvalue (`KismetArrayLibrary.Array_LastIndex` _webpoints_3))
  (if (`self.IsMeshGenerationPossible`)
    (`|ExecutionSequence`
      (:`then_0`
        (`self.ClearIndicators`)
        (bind _center (`self.GetCenterPoint`))
        (bind _output_get (set `self.Center` _center))
        (`KismetArrayLibrary.Array_Add` _webpoints_2 _output_get)
        ;[1 1 1] Set UV coordinates
        (`KismetArrayLibrary.Array_Resize` _uvs (`KismetArrayLibrary.Array_Length` _webpoints_2))
        (`KismetArrayLibrary.Array_Set` _uvs (`KismetArrayLibrary.Array_LastIndex` _uvs) (1.0 1.0))
        ;[1 1 1] Generate web mesh
        (bind _trianglevertices (`self.GetTriangleVertices`))
        (`PrimitiveComponent.SetMaterial` _proceduralmesh 0 (`self.DamagableWebMaterial`))
        (`ProceduralMeshComponent.CreateMeshSection_LinearColor` :`self` _proceduralmesh :`Vertices` (`self.WebPoints`) :`Triangles` _trianglevertices :`UV0` (`local.UVs`) :`bCreateCollision` true)
        (`GameplayStatics.PlaySoundAtLocation` "/Game/Dynamic/Sound/S_WebStructurePlace.S_WebStructurePlace" (`self.Center`) (struct) 1.0 1.0 0.0 null null null null)
        ;[1 1 1] Pop web center
        (`KismetArrayLibrary.Array_Remove` _webpoints (`KismetArrayLibrary.Array_LastIndex` _webpoints)))
      (:`then_1`
        ;[1 1 1] Add Lines between the triangles
        (for _index (range (+ _returnvalue 1))
          (bind _output (`|GetArrayItem` _webpoints_3 _index))
          (bind _cable (`self.CreateIndicator` (`|GetArrayItem` _webpoints_3 (mod (+ _index 1) _returnvalue)) _output))
          (`PrimitiveComponent.SetMaterial` _cable 0 "/Game/Static/Material/MI_Web.MI_Web")
          (`KismetArrayLibrary.Array_Add` (`self.IndicatorCables`) _cable)
          (bind _cable_2 (`self.CreateIndicator` (0.0 0.0 0.0) _output))
          (`PrimitiveComponent.SetMaterial` _cable_2 0 "/Game/Static/Material/MI_Web.MI_Web")
          (`KismetArrayLibrary.Array_Add` (`self.IndicatorCables`) _cable_2)
          (return (`self.GetConsumptionScore`)))))
    (else
      (`self.K2_DestroyActor`)
      (return 0.0))))

(fn `GetCenterPoint`
  (returns (Center :type "Vector Structure"))
  (locals (CenterPoint :type "Vector Structure"))
  (bind _webpoints (`self.WebPoints`))
  (bind _centerpoint (`local.CenterPoint`))
  ;[1 1 1] Get average of all the points
  (for _array_element _webpoints
    (set `local.CenterPoint` (+ _array_element _centerpoint)))
  (return (/ _centerpoint (`KismetArrayLibrary.Array_Length` _webpoints))))

(fn `GetConsumptionScore`
  (returns (ConsumptionScore :type "Float (double-precision)"))
  (locals (Score :type "Float (double-precision)"))
  (return (`KismetMathLibrary.Conv_IntToDouble` (`KismetArrayLibrary.Array_Length` (`self.WebPoints`)))))

(fn `GetTriangleVertices`
  (returns (TriangleVertices :type "Array of Integer"))
  (locals (Vertices :type "Array of Integer") (LastIdx :type Integer))
  (bind _vertices (`local.Vertices`))
  (bind _returnvalue (`KismetArrayLibrary.Array_Length` (`self.WebPoints`)))
  ;[1 1 1] Except the center
  (bind _output_get (set `local.LastIdx` (- _returnvalue 1)))
  (for _index (range (+ _output_get 1))
    ;[1 1 1] Add the triangle
    (`KismetArrayLibrary.Array_Add` _vertices _index)
    (`KismetArrayLibrary.Array_Add` _vertices (mod (+ _index 1) (- _returnvalue 1)))
    (`KismetArrayLibrary.Array_Add` _vertices (`local.LastIdx`)))
  (return (`local.Vertices`)))

(fn `IsMeshGenerationPossible`
  (returns (IsPossible :type Boolean))
  (return (> (`KismetArrayLibrary.Array_Length` (`self.WebPoints`)) 2)))

(fn `LocationInRange`
  (params (Location :type "Vector Structure"))
  (returns (InRange :type Boolean))
  (return (`self.ReachedMaxWebPoints`)))

(fn `ReachedMaxWebPoints`
  (returns (ReachedMaxWebPoints :type Boolean))
  (return (< (`KismetArrayLibrary.Array_Length` (`self.WebPoints`)) (`self.MaxPoints`))))

(fn `StartPlacement`
  (params (ImpactLocation :type "Vector Structure"))
  (`KismetArrayLibrary.Array_Add` (`self.WebPoints`) ImpactLocation)
  (`GameplayStatics.PlaySoundAtLocation` "/Game/Dynamic/Sound/S_WebStructureShoot.S_WebStructureShoot" ImpactLocation (struct) 1.0 1.0 0.0 null null null null))

(fn `UserConstructionScript`
  (`parent.UserConstructionScript`)
  (`PrimitiveComponent.SetMaterial` (`self.ProceduralMesh`) 0 (`self.DamagableWebMaterial`)))