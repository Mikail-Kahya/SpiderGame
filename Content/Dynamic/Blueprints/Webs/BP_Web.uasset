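; BP_Web is a base actor for destructible webs, with stub functions for placement, adding web, range checks and cleanup, presumably for child classes.
; Construction creates dynamic indicator and damageable materials and fills health.
; Damage lowers health and drives the damageable material's opacity and damage intensity.
; At zero health, Tick calls cleanup once, then delays destroying the actor so AI have time to untangle.
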(event `self.ReceiveTick`
  (params (DeltaSeconds :type "Float (single-precision)"))
  (bind _isdestroyed (`self.IsDestroyed`))
  (if _isdestroyed
    ;[1 1 1] Cleanup to give time for AI to untangle
    (if (`self.WebCleanedUp`)
      (bind _output_get (set `self.Timer` (+ (`self.Timer`) DeltaSeconds)))
      (if (> _output_get (`self.DestroyTime`))
        (`self.K2_DestroyActor`))
      (else
        (`self.CleanupWeb`)
        (set `self.WebCleanedUp` true)))))

(fn `Add Web`
  (params (Start :type "Vector Structure") (End :type "Vector Structure"))
  (returns (Finished :type Boolean))
  (return false))

(fn `AddToPlacement`
  (params (ImpactLocation :type "Vector Structure"))
  (returns (ConsumptionScore :type "Float (double-precision)"))
  (return 1.0))

(fn `CleanupWeb`)

(fn `DamageHealth`
  (params (Damage :type "Float (double-precision)"))
  (set `self.Health` (- (`self.Health`) Damage))
  (`self.ShowDamage`))

(fn `EndPlacement`
  (params (ImpactLocation :type "Vector Structure"))
  (returns (ConsumptionScore :type "Float (double-precision)"))
  (return 0.0))

(fn `GetConsumptionScore`
  (returns (ConsumptionScore :type "Float (double-precision)"))
  (return 1.0))

(fn `IsDestroyed`
  (returns (IsDestroyed :type Boolean))
  (return (<= (`self.Health`) 0.0)))

(fn `LocationInRange`
  (params (Location :type "Vector Structure"))
  (returns (InRange :type Boolean))
  (return false))

(fn `PlayDestructionSound`
  (params (Location :type "Vector Structure"))
  (`GameplayStatics.PlaySoundAtLocation` "/Game/Dynamic/Sound/S_WebDestroy.S_WebDestroy" Location (struct) 1.0 1.0 0.0 null null null null))

(fn `ShowDamage`
  (bind _damagablewebmaterial (`self.DamagableWebMaterial`))
  (bind _returnvalue (/ (`self.Health`) (`self.MaxHealth`)))
  (`MaterialInstanceDynamic.SetScalarParameterValue` _damagablewebmaterial "Opacity" _returnvalue)
  (`MaterialInstanceDynamic.SetScalarParameterValue` _damagablewebmaterial "DamageIntensity" (* (- 1.0 _returnvalue) 2.0)))

(fn `StartPlacement`
  (params (ImpactLocation :type "Vector Structure")))

(fn `UpdatePlacement`
  (params (ImpactLocation :type "Vector Structure")))

(fn `UserConstructionScript`
  (bind _returnvalue (`KismetMaterialLibrary.CreateDynamicMaterialInstance` "/Game/Static/Material/MI_WebTranslucent.MI_WebTranslucent"))
  (set `self.IndicatorMaterial` _returnvalue)
  (bind _returnvalue_2 (`KismetMaterialLibrary.CreateDynamicMaterialInstance` "/Game/Static/Material/MI_Web.MI_Web"))
  (set `self.DamagableWebMaterial` _returnvalue_2)
  (set `self.Health` (`self.MaxHealth`)))