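; BP_WebLine is a placeable web that spans a straight line between two points, with a flat consumption score.
; During placement a cable indicator stretches from start to aim point, turning green or red by the end point's range from the player pawn.
; An in-range release builds a rotated procedural box mesh with collision and damageable web material along the line.
; Sounds play on shoot, placement and cleanup, which destroys indicator and mesh.
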(fn `Add Web`
  (params (Start :type "Vector Structure") (End :type "Vector Structure"))
  (returns (Finished :type Boolean))
  (return false))

(fn `AddToPlacement`
  (params (ImpactLocation :type "Vector Structure"))
  (returns (ConsumptionScore :type "Float (double-precision)"))
  (set `self.End` ImpactLocation)
  (return 0.0))

(fn `CleanupWeb`
  (`ActorComponent.K2_DestroyComponent` (`self.Indicator`))
  (`ActorComponent.K2_DestroyComponent` (`self.ProceduralMesh`))
  (`self.PlayDestructionSound` (`self.GetWebCenter`)))

(fn `EndPlacement`
  (params (ImpactLocation :type "Vector Structure"))
  (returns (ConsumptionScore :type "Float (double-precision)"))
  (locals (Score :type "Float (double-precision)"))
  (bind _start (`self.Start`))
  (bind _websize (`self.WebSize`))
  (if (`self.LocationInRange` ImpactLocation)
    (bind _output_get (set `self.End` ImpactLocation))
    (set `local.Score` (`self.GetConsumptionScore`))
    ;[1 1 1] Generate procedural mesh
    (bind _returnvalue (`AddComponent|NODE_AddProceduralMeshComponent-5` :`RelativeTransform` (`KismetMathLibrary.MakeTransform` _start (`KismetMathLibrary.Quat_Rotator` (`KismetMathLibrary.Quat_FindBetweenVectors` (`KismetMathLibrary.Vector_Up`) (`KismetMathLibrary.Normal` (- ImpactLocation _start)))))))
    (`PrimitiveComponent.SetMaterial` _returnvalue 0 (`self.DamagableWebMaterial`))
    (bind (_vertices _triangles _normals _uvs _tangents) (`KismetProceduralMeshLibrary.GenerateBoxMesh` (`KismetMathLibrary.MakeVector` _websize _websize (`KismetMathLibrary.Vector_Distance` _output_get _start))))
    (`ProceduralMeshComponent.CreateMeshSection_LinearColor` :`self` _returnvalue :`Vertices` _vertices :`Triangles` _triangles :`Normals` _normals :`UV0` _uvs :`Tangents` _tangents :`bCreateCollision` true)
    (`GameplayStatics.PlaySoundAtLocation` "/Game/Dynamic/Sound/S_WebLinePlace.S_WebLinePlace" (`self.GetWebCenter`) (struct) 1.0 1.0 0.0 null null null null))
  (`SceneComponent.SetVisibility` (`self.Indicator`) false true)
  (return (`local.Score`)))

(fn `GetConsumptionScore`
  (returns (ConsumptionScore :type "Float (double-precision)"))
  (locals (ScoreMaxRange :type "Float (double-precision)" :default 10000.0))
  (return 1.0))

(fn `GetWebCenter`
  (returns (Center :type "Vector Structure"))
  (bind _start (`self.Start`))
  (return (+ (* (- (`self.End`) _start) 2.0) _start)))

(fn `LocationInRange`
  (params (Location :type "Vector Structure"))
  (returns (InRange :type Boolean))
  (return (< (`KismetMathLibrary.Vector_DistanceSquared` (`self.K2_GetActorLocation` (`GameplayStatics.GetPlayerPawn` 0)) Location) (`KismetMathLibrary.Square` (`self.PlacementRange`)))))

(fn `StartPlacement`
  (params (ImpactLocation :type "Vector Structure"))
  (bind _indicator (`self.Indicator`))
  (`SceneComponent.SetVisibility` _indicator true false)
  (`SceneComponent.K2_SetWorldLocation` _indicator ImpactLocation false false)
  (bind _output_get (set `self.Start` ImpactLocation))
  (`GameplayStatics.PlaySoundAtLocation` "/Game/Dynamic/Sound/S_WebLineShoot.S_WebLineShoot" _output_get (struct) 1.0 1.0 0.0 null null null null))

(fn `UpdatePlacement`
  (params (ImpactLocation :type "Vector Structure"))
  (bind _indicatormaterial (`self.IndicatorMaterial`))
  (bind _output_get (set `CableComponent.EndLocation` ImpactLocation (`self.Indicator`)))
  (if (`self.LocationInRange` _output_get)
    (`MaterialInstanceDynamic.SetVectorParameterValue` _indicatormaterial "Color" (struct :`G` 1.0 :`B` 0.035646 :`A` 1.0))
    (else
      (`MaterialInstanceDynamic.SetVectorParameterValue` _indicatormaterial "Color" (struct :`R` 1.0 :`G` 0.02448 :`A` 1.0)))))

(fn `UserConstructionScript`
  (bind _indicator (`self.Indicator`))
  (`parent.UserConstructionScript`)
  (set `CableComponent.CableWidth` (`self.WebSize`) _indicator)
  (`PrimitiveComponent.SetMaterial` _indicator 0 (`self.IndicatorMaterial`)))