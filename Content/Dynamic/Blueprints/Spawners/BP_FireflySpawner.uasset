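; Spawner that creates AI fireflies at the start of a spline path while the world count is below the game mode's MaxFireflies.
; Each firefly runs BT_Firefly and receives the spawner reference plus a fly speed randomized once per spawner at BeginPlay.
; GetTarget supplies points at a given spline distance, randomly strayed along the right vector and world X.
; The construction script tints the path visuals.
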(event `self.ReceiveBeginPlay`
  (set `self.FlySpeed` (`KismetMathLibrary.RandomFloatInRange` (`self.MinFlySpeed`) (`self.MaxFlySpeed`))))

(event `Spawn`
  (bind (_randomlocation _splinerotation) (`self.GetRandomPointAlongSpline` 0.0))
  (bind _outactors (`GameplayStatics.GetAllActorsOfClass` "/Game/Dynamic/Blueprints/Pawns/Fireflies/BP_BaseFirefly.BP_BaseFirefly_C"))
  (if (< (`KismetArrayLibrary.Array_Length` _outactors) (`/Game/Dynamic/Blueprints/GameMode/BP_SpiderGameMode.MaxFireflies` (cast `/Game/Dynamic/Blueprints/GameMode/BP_SpiderGameMode` (`GameplayStatics.GetGameMode`) :!pure true)))
    (bind _returnvalue (`AIBlueprintHelperLibrary.SpawnAIFromClass` "/Game/Dynamic/Blueprints/Pawns/Fireflies/BP_BaseFirefly.BP_BaseFirefly_C" "/Game/Dynamic/Blueprints/Pawns/Fireflies/BehaviorTree/BT_Firefly.BT_Firefly" _randomlocation _splinerotation false null))
    (message `/Game/Dynamic/Blueprints/Interfaces/BPI_FlyPath.SetMovementSpeed` _returnvalue (`self.FlySpeed`))
    (message `/Game/Dynamic/Blueprints/Interfaces/BPI_FlyPath.SetSpawner` _returnvalue self)))

(fn `GetRandomPointAlongSpline`
  (params (SplineDistanceTravelled :type "Float (double-precision)"))
  (returns (RandomLocation :type "Vector Structure") (SplineRotation :type "Rotator Structure"))
  (bind _path (`self.Path`))
  (bind _strayradius (`self.StrayRadius`))
  (bind _strayradius_2 (`self.StrayRadius`))
  (return (+ (`SplineComponent.GetLocationAtDistanceAlongSpline` _path SplineDistanceTravelled "World") (* (`SplineComponent.GetRightVectorAtDistanceAlongSpline` _path SplineDistanceTravelled "World") (`KismetMathLibrary.RandomFloatInRange` (* _strayradius_2 -1.0) _strayradius_2)) (`KismetMathLibrary.MakeVector` (`KismetMathLibrary.RandomFloatInRange` (* _strayradius -1.0) _strayradius))) (`SplineComponent.GetRotationAtDistanceAlongSpline` _path SplineDistanceTravelled "World")))

(fn `GetTarget`
  (params (DistanceTravelled :type "Float (double-precision)"))
  (returns (Target :type "Vector Structure") (SplineRotation :type "Rotator Structure"))
  (bind (_randomlocation _splinerotation) (`self.GetRandomPointAlongSpline` DistanceTravelled))
  (return _randomlocation _splinerotation))

(fn `UserConstructionScript`
  (`NiagaraComponent.SetVariableLinearColor` (`self.PathVisuals`) "Color" (`self.VisualsColor`)))