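; AI controller for firefly pawns that runs the BT_Firefly behavior tree on BeginPlay.
; On possess it seeds the blackboard with the pawn's location as target and a zero direction.
; Spawner and movement speed setter events pass their values into the blackboard.
; GetTarget takes a distance travelled but is a stub returning zero target and spline rotation.
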(event `self.ReceivePossess`
  (params (PossessedPawn :type "Pawn Object Reference"))
  (`self.SetStartValues` PossessedPawn))

(event `self.ReceiveBeginPlay`
  (`self.RunBehaviorTree` "/Game/Dynamic/Blueprints/Pawns/Fireflies/BehaviorTree/BT_Firefly.BT_Firefly"))

(event `/Game/Dynamic/Blueprints/Interfaces/BPI_FlyPath.SetSpawner`
  (params (Spawner :type "Actor Object Reference"))
  (`BlackboardComponent.SetValueAsObject` (`AIBlueprintHelperLibrary.GetBlackboard` null) (`self.SpawnerKey`) Spawner))

(event `/Game/Dynamic/Blueprints/Interfaces/BPI_FlyPath.SetMovementSpeed`
  (params (MovementSpeed :type "Float (double-precision)"))
  (`BlackboardComponent.SetValueAsFloat` (`AIBlueprintHelperLibrary.GetBlackboard` null) (`self.MovementSpeedKey`) MovementSpeed))

(fn `GetTarget`
  (params (DistanceTravelled :type "Float (double-precision)"))
  (returns (Target :type "Vector Structure") (SplineRotation :type "Rotator Structure"))
  (return (0.0 0.0 0.0)))

(fn `SetStartValues`
  (params (PossessedPawn :type "Pawn Object Reference"))
  (locals (TargetKey :type Name :default "Target") (DirectionKey :type Name :default "Direction"))
  (bind _returnvalue (`AIBlueprintHelperLibrary.GetBlackboard` null))
  (`BlackboardComponent.SetValueAsVector` _returnvalue (`local.TargetKey`) (`self.K2_GetActorLocation` PossessedPawn))
  (`BlackboardComponent.SetValueAsVector` _returnvalue (`local.DirectionKey`) (0.0 0.0 0.0)))

(fn `UserConstructionScript`)