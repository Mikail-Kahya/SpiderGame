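; Base firefly pawn, the spider's consumable prey, which reports being consumed or destroyed to BP_SpiderGameMode.
; Tick flaps mirrored wings via a timeline, applies swept movement from behavior-tree input, and reverts highlights after a delay to default or stuck-in-web material from the blackboard.
; Spawner and speed settings are forwarded to the controller, while GetTarget is a zero-returning stub, apparently for subclasses to override.
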(event `self.ReceiveTick`
  (params (DeltaSeconds :type "Float (single-precision)"))
  (`|ExecutionSequence`
    (:`then_0`
      ;[1 1 1] Flap wings
      (bind (_direction _wingflap) (`Timeline|WingFlap` :`NewTime` DeltaSeconds)
        (:`Update`
          (bind _returnvalue (* _wingflap (`self.WingRotation`)))
          (`SceneComponent.K2_SetRelativeRotation` (`self.Firefly_BackWing1`) (`KismetMathLibrary.MakeRotator` _returnvalue) false false)
          (`SceneComponent.K2_SetRelativeRotation` (`self.Firefly_FrontWing1`) (`KismetMathLibrary.MakeRotator` _returnvalue) false false)
          (`SceneComponent.K2_SetRelativeRotation` (`self.Firefly_MiddleWing`) (`KismetMathLibrary.MakeRotator` _returnvalue) false false)
          (`SceneComponent.K2_SetRelativeRotation` (`self.Firefly_MiddleWing1`) (`KismetMathLibrary.MakeRotator` (* _returnvalue -1.0)) false false)
          (`SceneComponent.K2_SetRelativeRotation` (`self.Firefly_FrontWing`) (`KismetMathLibrary.MakeRotator` (* _returnvalue -1.0)) false false)
          (`SceneComponent.K2_SetRelativeRotation` (`self.Firefly_BackWing`) (`KismetMathLibrary.MakeRotator` (* _returnvalue -1.0)) false false))))
    (:`then_1`
      ;[1 1 1] Move forward (velocity calculated in behavior tree)
      (bind _returnvalue_2 (`self.ConsumeMovementInputVector`))
      (`self.K2_AddActorWorldOffset` (* _returnvalue_2 DeltaSeconds 4.0) true true))
    (:`then_2`
      (if (`self.Highlighted`)
        (`KismetSystemLibrary.Delay` 0.5)
        (`self.UpdateMaterial`)))))

(event `/Game/Dynamic/Blueprints/Interfaces/BPI_HuntInterface.Highlight`
  (`PrimitiveComponent.SetMaterial` (`self.Firefly_Firefly1`) 0 (`self.HighlightedMat`))
  (set `self.Highlighted` true))

(event `/Game/Dynamic/Blueprints/Interfaces/BPI_HuntInterface.Consume`
  (`self.K2_DestroyActor` (`self.GetController`))
  (`self.K2_DestroyActor`)
  (bind _asbp_spider_game_mode (cast `/Game/Dynamic/Blueprints/GameMode/BP_SpiderGameMode` (`GameplayStatics.GetGameMode`)))
  (`/Game/Dynamic/Blueprints/GameMode/BP_SpiderGameMode.FlyConsumed` _asbp_spider_game_mode))

(event `/Game/Dynamic/Blueprints/Interfaces/BPI_FlyPath.SetSpawner`
  (params (Spawner :type "Actor Object Reference"))
  (message `/Game/Dynamic/Blueprints/Interfaces/BPI_FlyPath.SetSpawner` (`self.GetController`) Spawner))

(event `/Game/Dynamic/Blueprints/Interfaces/BPI_FlyPath.SetMovementSpeed`
  (params (MovementSpeed :type "Float (double-precision)"))
  (message `/Game/Dynamic/Blueprints/Interfaces/BPI_FlyPath.SetMovementSpeed` (`self.GetController`) MovementSpeed))

(event `self.ReceiveDestroyed`
  (bind _asbp_spider_game_mode (cast `/Game/Dynamic/Blueprints/GameMode/BP_SpiderGameMode` (`GameplayStatics.GetGameMode`)))
  (`/Game/Dynamic/Blueprints/GameMode/BP_SpiderGameMode.FlyDied` _asbp_spider_game_mode))

(fn `GetTarget`
  (params (DistanceTravelled :type "Float (double-precision)"))
  (returns (Target :type "Vector Structure") (SplineRotation :type "Rotator Structure"))
  (return (0.0 0.0 0.0)))

(fn `UpdateMaterial`
  (bind _firefly_firefly1 (`self.Firefly_Firefly1`))
  (if (`BlackboardComponent.GetValueAsBool` (`AIBlueprintHelperLibrary.GetBlackboard` null) (`self.BBStuckInWeb`))
    (`PrimitiveComponent.SetMaterial` _firefly_firefly1 0 (`self.StuckInWebMat`))
    (set `self.Highlighted` false)
    (else
      (`PrimitiveComponent.SetMaterial` _firefly_firefly1 0 (`self.DefaultMat`)))))

(fn `UserConstructionScript`)