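; Base player spider pawn that shoots web lines, builds multi-point web structures and eats fireflies.
; It adds WebShooter, WebCreator and Hunger components at BeginPlay; shooter traces feed points and placement previews to the creator.
; Spawned webs cost hunger scaled by the creator's consumption score, while eating overlapping fireflies notifies Hunger.
; Mounting passes web line endpoints to C++ movement, and death notifies the game mode.
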(event `self.ReceiveBeginPlay`
  (`|ExecutionSequence`
    (:`then_0`
      ;[1 1 1] Add Input Context map
      (bind _asplayer_controller (cast `PlayerController` (`self.GetController`)))
      (bind _returnvalue (pcsubsystem `EnhancedInputLocalPlayerSubsystem` _asplayer_controller))
      (`/Engine/EditorBlueprintResources/StandardMacros.IsValid` _returnvalue
        (:`Is Valid`
          (`EnhancedInputSubsystemInterface.AddMappingContext` _returnvalue "/Game/Dynamic/Blueprints/Pawns/Player/Input/IMC_Gameplay.IMC_Gameplay" 0 (struct)))))
    (:`then_1`
      ;[1 1 1] Setup web creator / spawner
      (bind _returnvalue_2 (`|AddComponentByClass` "/Game/Dynamic/Blueprints/Pawns/Player/Components/BPC_WebCreator.BPC_WebCreator_C"))
      (bind _output_get (set `self.WebCreator` _returnvalue_2))
      (`/Game/Dynamic/Blueprints/Pawns/Player/Components/BPC_WebCreator.Setup` _output_get)
      ;[1 1 1] Setup Web shooter
      (bind _returnvalue_3 (`|AddComponentByClass` "/Game/Dynamic/Blueprints/Pawns/Player/Components/BPC_WebShooter.BPC_WebShooter_C"))
      (bind _output_get_2 (set `self.WebShooter` _returnvalue_3))
      (set `/Game/Dynamic/Blueprints/Pawns/Player/Components/BPC_WebShooter.WebMaxRange` 20000.0 _output_get_2)
      ;[1 1 1] Add hunger
      (bind _returnvalue_4 (`|AddComponentByClass` "/Game/Dynamic/Blueprints/Pawns/Player/Components/BPC_Hunger.BPC_Hunger_C"))
      (set `self.Hunger` _returnvalue_4))))

(event `self.ReceiveTick`
  (params (DeltaSeconds :type "Float (single-precision)"))
  (bind (_inrange _fireflies) (`self.FliesInRange`))
  (bind _websocket (`self.WebSocket`))
  (`|ExecutionSequence`
    (:`then_0`
      ;[1 1 1] Web feedback
      (bind (_isvalid _impactlocation) (`/Game/Dynamic/Blueprints/Interfaces/BPI_WebShooterInterface.PointIsValid` (`self.WebShooter`) (`SceneComponent.GetForwardVector` _websocket) (`SceneComponent.K2_GetComponentLocation` _websocket)))
      (`/Game/Dynamic/Blueprints/Pawns/Player/Components/BPC_WebCreator.Update` (`self.WebCreator`) _impactlocation)
      ;;[1 1 1] Update the crosshair by validity
      (if (`self.WebHit`)
        (bind _isvalid_2 (`/Game/Dynamic/Blueprints/Pawns/Player/Components/BPC_WebCreator.IsValidPlacement` (`self.WebCreator`) _impactlocation))
        (set `self.ValidWebPlacement` (and _isvalid_2 _isvalid))
        (else
          (set `self.ValidWebPlacement` _isvalid))))
    (:`then_1`
      (if _inrange
        (for _array_element _fireflies
          (message `/Game/Dynamic/Blueprints/Interfaces/BPI_HuntInterface.Highlight` _array_element))))))

(event `self.ReceiveDestroyed`
  (`/Game/Dynamic/Blueprints/Pawns/Player/Components/BPC_WebCreator.CancelWeb` (`self.WebCreator`)))

(event `self.MountWebLine`
  (params (SurfaceActorPtr :type "Actor Object Reference"))
  ;[1 1 1] Interact with the C++ to set the movement target points
  (`/Engine/EditorBlueprintResources/StandardMacros.IsValid` SurfaceActorPtr
    (:`Is Valid`
      (bind _asbp_web_line (cast `/Game/Dynamic/Blueprints/Webs/BP_WebLine` SurfaceActorPtr))
      (`self.SetClosestWeb` (`/Game/Dynamic/Blueprints/Webs/BP_WebLine.Start` _asbp_web_line) (`/Game/Dynamic/Blueprints/Webs/BP_WebLine.End` _asbp_web_line)))))

(event `ShootWebLine`
  ;[0 0.7713 1] Shoot WebLine
  (if (not (`self.WebHit`))
    (bind (_didhit _impactlocation) (`self.UseWebShooter`))
    (bind _output_get (set `self.WebHit` _didhit))
    (if _output_get
      (`/Game/Dynamic/Blueprints/Pawns/Player/Components/BPC_WebCreator.AddPoint` (`self.WebCreator`) _impactlocation))))

(event `ReleaseWebLine`
  (params (SpawnWebLine :type Boolean))
  (bind _webcreator (`self.WebCreator`))
  ;[0.01319 0.7346 1] Release WebLine
  (`|ExecutionSequence`
    (:`then_0`
      ;;[1 1 1] Check if webline can be released
      (if (and SpawnWebLine (`self.WebHit`) (`/Game/Dynamic/Blueprints/Pawns/Player/Components/BPC_WebCreator.InProcessOfCreating` _webcreator) (`/Game/Dynamic/Blueprints/Pawns/Player/Components/BPC_WebCreator.ShootWebLine` _webcreator))
        (bind (_didhit _impactlocation) (`self.UseWebShooter`))
        ;;[1 1 1] Spawn web line
        (if _didhit
          (`/Game/Dynamic/Blueprints/Pawns/Player/Components/BPC_WebCreator.SpawnWeb` (`self.WebCreator`) _impactlocation)
          ;;[1 1 1] Reduce food in price for the web
          (`/Game/Dynamic/Blueprints/Interfaces/BPI_HuntInterface.HungerOut` (`self.Hunger`) (`self.GetFoodReduction`)))
        (else
          (`/Game/Dynamic/Blueprints/Pawns/Player/Components/BPC_WebCreator.CancelWeb` (`self.WebCreator`))
          (`GameplayStatics.PlaySound2D` "/Game/Dynamic/Sound/S_CancelWebLine.S_CancelWebLine" 1.0 1.0 0.0 null null))))
    (:`then_1`
      (set `self.WebHit` false))))

(event `ActivateWebStructure`
  ;[0.8937 0.1546 1] Start WebStructure
  (`/Game/Dynamic/Blueprints/Pawns/Player/Components/BPC_WebCreator.CancelWeb` (`self.WebCreator`))
  (set `self.WebHit` true)
  (`/Game/Dynamic/Blueprints/Pawns/Player/Components/BPC_WebCreator.SetWebType` (`self.WebCreator`) false)
  (`GameplayStatics.PlaySound2D` "/Game/Dynamic/Sound/S_StartWebStructure.S_StartWebStructure" 1.0 1.0 0.0 null null))

(event `DeactivateWebStructure`
  (params (SpawnWebStucture :type Boolean))
  (bind _webcreator (`self.WebCreator`))
  ;[0.9972 0.2519 1] Deactivate WebStructure
  (`|ExecutionSequence`
    (:`then_0`
      ;;[1 1 1] Check if WebStructure can be deactivated
      (if (and SpawnWebStucture (`self.WebHit`) (`/Game/Dynamic/Blueprints/Pawns/Player/Components/BPC_WebCreator.InProcessOfCreating` _webcreator) (not (`/Game/Dynamic/Blueprints/Pawns/Player/Components/BPC_WebCreator.ShootWebLine` _webcreator)))
        (`/Game/Dynamic/Blueprints/Pawns/Player/Components/BPC_WebCreator.SpawnWeb` (`self.WebCreator`) (0.0 0.0 0.0))
        (`GameplayStatics.PlaySound2D` "/Game/Dynamic/Sound/S_PlaceWebStructure.S_PlaceWebStructure" 1.0 1.0 0.0 null null)
        ;;[1 1 1] Reduce food in price for the web
        (`/Game/Dynamic/Blueprints/Interfaces/BPI_HuntInterface.HungerOut` (`self.Hunger`) (`self.GetFoodReduction`))
        (else
          (`/Game/Dynamic/Blueprints/Pawns/Player/Components/BPC_WebCreator.CancelWeb` (`self.WebCreator`))
          (`GameplayStatics.PlaySound2D` "/Game/Dynamic/Sound/S_CancelWebStructure.S_CancelWebStructure" 1.0 1.0 0.0 null null))))
    (:`then_1`
      (`/Game/Dynamic/Blueprints/Pawns/Player/Components/BPC_WebCreator.SetWebType` (`self.WebCreator`) true)
      (set `self.WebHit` false))))

(event `AddPointToWebStructure`
  ;[1 0.2354 0.9889] Add point to WebStructure
  (bind (_didhit _impactlocation) (`self.UseWebShooter`))
  (if _didhit
    (`/Game/Dynamic/Blueprints/Pawns/Player/Components/BPC_WebCreator.AddPoint` (`self.WebCreator`) _impactlocation)))

(event `EatBug`
  (bind (_inrange _fireflies) (`self.FliesInRange`))
  ;[0.3547 1 0.2604] Eat
  (if _inrange
    (for _array_element _fireflies
      (message `/Game/Dynamic/Blueprints/Interfaces/BPI_HuntInterface.Consume` _array_element)
      (message `/Game/Dynamic/Blueprints/Interfaces/BPI_HuntInterface.Consume` (`self.Hunger`))
      (`GameplayStatics.PlaySoundAtLocation` "/Game/Dynamic/Sound/S_Eat.S_Eat" (`self.K2_GetActorLocation`) (struct) 1.0 1.0 0.0 null null null null))))

(event `/Game/Dynamic/Blueprints/Interfaces/BPI_HuntInterface.Died`
  (`/Game/Dynamic/Blueprints/Pawns/Player/Components/BPC_WebCreator.CancelWeb` (`self.WebCreator`))
  (bind _asbp_spider_game_mode (cast `/Game/Dynamic/Blueprints/GameMode/BP_SpiderGameMode` (`GameplayStatics.GetGameMode`)))
  (`/Game/Dynamic/Blueprints/GameMode/BP_SpiderGameMode.PlayerDeath` _asbp_spider_game_mode))

(fn `FliesInRange`
  (returns (InRange :type Boolean) (FireFlies :type "Array of Actor Object Reference"))
  (bind _overlappingactors (`PrimitiveComponent.GetOverlappingActors` (`self.ConsumptionCollider`) "/Game/Dynamic/Blueprints/Pawns/Fireflies/BP_BaseFirefly.BP_BaseFirefly_C"))
  (return (`KismetArrayLibrary.Array_IsNotEmpty` _overlappingactors) _overlappingactors))

(fn `GetFoodReduction`
  (returns (`Food Reduction` :type "Float (double-precision)"))
  (locals (Scalar :type "Float (double-precision)" :default 5.0))
  (return (* (`/Game/Dynamic/Blueprints/Pawns/Player/Components/BPC_WebCreator.ConsumptionScore` (`self.WebCreator`)) (`local.Scalar`))))

(fn `UserConstructionScript`)

(fn `UseWebShooter`
  (returns (DidHit :type Boolean) (ImpactLocation :type "Vector Structure"))
  (bind (_hit _impactpoint) (`/Game/Dynamic/Blueprints/Interfaces/BPI_WebShooterInterface.Shoot` (`self.WebShooter`) (`SceneComponent.GetForwardVector` (`self.Camera`)) (`SceneComponent.K2_GetComponentLocation` (`self.WebSocket`))))
  (return _hit _impactpoint))