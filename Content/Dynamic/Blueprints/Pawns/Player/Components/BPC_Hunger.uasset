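; Player hunger component that tracks a food level and notifies the player pawn of death when it runs out.
; Food starts at MaxFood, drains by HungerRate each Tick, and sends DiedMessage on every Tick it is at zero.
; Consume and HungerOut raise or lower it through AddFood, which clamps to a hardcoded 0–100 range.
; GetHungerPercentage exposes Food as a fraction of MaxFood.
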(event `self.ReceiveBeginPlay`
  (set `self.Food` (`self.MaxFood`)))

(event `self.ReceiveTick`
  (params (DeltaSeconds :type "Float (single-precision)"))
  ;[1 1 1] Degrade food
  (`self.AddFood` (* DeltaSeconds (`self.HungerRate`) -1.0))
  ;[1 1 1] Die
  (if (<= (`self.Food`) 0.0)
    (message `/Game/Dynamic/Blueprints/Interfaces/BPI_HuntInterface.Died` (`GameplayStatics.GetPlayerPawn` 0))))

(event `/Game/Dynamic/Blueprints/Interfaces/BPI_HuntInterface.Consume`
  (`self.AddFood` (`self.ReplenishAmount`)))

(event `/Game/Dynamic/Blueprints/Interfaces/BPI_HuntInterface.HungerOut`
  (params (FoodReduction :type "Float (double-precision)"))
  (`self.AddFood` (* FoodReduction -1.0)))

(fn `AddFood`
  (params (AddedFood :type "Float (double-precision)"))
  (set `self.Food` (`KismetMathLibrary.FClamp` (+ AddedFood (`self.Food`)) 0.0 100.0)))

(fn `GetHungerPercentage`
  (returns (Percentage :type "Float (double-precision)"))
  (return (/ (`self.Food`) (`self.MaxFood`))))