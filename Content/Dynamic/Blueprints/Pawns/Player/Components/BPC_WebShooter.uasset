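; Player web shooter component that finds and reports the endpoints of webs between surfaces.
; All queries share one Visibility line trace up to a max range, with the impact point shifted along the aim direction by a margin.
; Shoot stores the first point, Release traces again and returns both ends with validity, and PointIsValid checks aim without storing.
; Reel is an empty stub, and nothing here spawns a web.
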(event `/Game/Dynamic/Blueprints/Interfaces/BPI_WebShooterInterface.Reel`
  (params (Direction :type "Float (double-precision)")))

(fn `CheckValidWeb`
  (params (Direction :type "Vector Structure") (Location :type "Vector Structure"))
  (returns (DidHit :type Boolean) (ImpactPoint :type "Vector Structure"))
  ;[1 1 1] Raycast max range
  (bind _outhit (`KismetSystemLibrary.LineTraceSingle` Location (+ Location (* Direction (`self.WebMaxRange`))) "TraceTypeQuery1"))
  (bind (_bblockinghit _binitialoverlap _time _distance _location _impactpoint) (`GameplayStatics.BreakHitResult` _outhit))
  (return _bblockinghit (+ _impactpoint (* Direction (`self.WebMargin`)))))

(fn `PointIsValid`
  (params (Direction :type "Vector Structure") (Location :type "Vector Structure"))
  (returns (IsValid :type Boolean) (ImpactLocation :type "Vector Structure"))
  (bind (_didhit _impactpoint) (`self.CheckValidWeb` Direction Location))
  (return _didhit _impactpoint))

(fn `Release`
  (params (LookDirection :type "Vector Structure") (Location :type "Vector Structure"))
  (returns (WebTo :type "Vector Structure") (WebFrom :type "Vector Structure") (IsValid :type Boolean))
  (bind (_didhit _impactpoint) (`self.CheckValidWeb` LookDirection Location))
  (return (`self.WebPoint`) _impactpoint _didhit))

(fn `Shoot`
  (params (Direction :type "Vector Structure") (Location :type "Vector Structure"))
  (returns (Hit :type Boolean) (ImpactPoint :type "Vector Structure"))
  (bind (_didhit _impactpoint) (`self.CheckValidWeb` Direction Location))
  (bind _output_get (set `self.WebPoint` _impactpoint))
  (return _didhit _output_get))