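; Player pawn component that manages placing spider webs, either as a web line or a web structure.
; The first added point spawns the chosen web actor and starts placement, and later points extend it until it is finalized or cancelled.
; It forwards impact locations to the web for preview updates and range checks, and tracks the consumption score the web reports.
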(event `AddPoint`
  (params (ImpactLocation :type "Vector Structure"))
  (if (`self.InProcessOfCreating`)
    ;[1 1 1] Add point to web
    (bind _consumptionscore (`/Game/Dynamic/Blueprints/Webs/BP_Web.AddToPlacement` (`self.Web`) ImpactLocation))
    (set `self.ConsumptionScore` _consumptionscore)
    (else
      ;[1 1 1] Setup new web
      (bind _newparam (`self.Make New Web`))
      (`/Game/Dynamic/Blueprints/Webs/BP_Web.StartPlacement` _newparam ImpactLocation)
      (set `self.InProcessOfCreating` true))))

(event `Update`
  (params (ImpactLocation :type "Vector Structure"))
  (bind _web (`self.Web`))
  (if (and (`self.InProcessOfCreating`) (`KismetSystemLibrary.IsValid` (`self.Web`)))
    (`/Game/Dynamic/Blueprints/Webs/BP_Web.UpdatePlacement` _web ImpactLocation)
    (set `self.ConsumptionScore` (`/Game/Dynamic/Blueprints/Webs/BP_Web.GetConsumptionScore` _web))
    (else
      (set `self.ConsumptionScore` 0.0))))

(event `SpawnWeb`
  (params (ImpactLocation :type "Vector Structure"))
  (bind _consumptionscore (`/Game/Dynamic/Blueprints/Webs/BP_Web.EndPlacement` (`self.Web`) ImpactLocation))
  (set `self.ConsumptionScore` _consumptionscore)
  (set `self.Web` null)
  (set `self.InProcessOfCreating` false))

(event `CancelWeb`
  (bind _web (`self.Web`))
  (if (`KismetSystemLibrary.IsValid` _web)
    (`Actor.K2_DestroyActor` _web))
  (set `self.InProcessOfCreating` false)
  (set `self.ConsumptionScore` 0.0))

(fn `IsValidPlacement`
  (params (ImpactLocation :type "Vector Structure"))
  (returns (IsValid :type Boolean))
  (return (`/Game/Dynamic/Blueprints/Webs/BP_Web.LocationInRange` (`self.Web`) ImpactLocation)))

(fn `Make New Web`
  (returns (NewParam :type "/Game/Dynamic/Blueprints/Webs/BP_Web Object Reference"))
  (if (`self.ShootWebLine`)
    ;[1 1 1] Create Web line
    (bind _returnvalue (`|SpawnActorFromClass` "/Game/Dynamic/Blueprints/Webs/BP_WebLine.BP_WebLine_C" (`KismetMathLibrary.MakeTransform` (0.0 0.0 0.0)) "AlwaysSpawn" "MultiplyWithRoot" null null))
    (bind _output_get (set `self.Web` _returnvalue))
    (return _output_get)
    (else
      ;[1 1 1] Create Web structure
      (bind _returnvalue_2 (`|SpawnActorFromClass` "/Game/Dynamic/Blueprints/Webs/BP_WebStructure.BP_WebStructure_C" (`KismetMathLibrary.MakeTransform` (0.0 0.0 0.0)) "AlwaysSpawn" "MultiplyWithRoot" null null))
      (bind _output_get_2 (set `self.Web` _returnvalue_2))
      (return _output_get_2))))

(fn `Setup`
  (`self.Make New Web`))

(fn `SetWebType`
  (params (WebLine :type Boolean))
  (bind _web (`self.Web`))
  (`|ExecutionSequence`
    (:`then_0`
      (set `self.ShootWebLine` WebLine)
      (`/Engine/EditorBlueprintResources/StandardMacros.IsValid` _web
        (:`Is Valid`
          (if (`/Game/Dynamic/Blueprints/Webs/BP_Web.WebPlaced` _web)
            (`Actor.K2_DestroyActor` _web)))))
    (:`then_1`
      (`self.Make New Web`))))