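; Game mode for the spider game that tracks survival time and fly death/consumption counts, starts firefly spawning, and handles respawn and death.
; On begin play it gives each BP_FireflySpawner an immediate spawn and a looping timer with a randomly chosen interval.
; Respawn replaces the pawn at a player start, carrying the Hunger component's food value across.
; Player death pauses the game and shows the end screen in UI-only input mode.
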(event `self.ReceiveBeginPlay`
  (bind _returnvalue (`GameplayStatics.GetPlayerController` 0))
  (set `PlayerController.bShowMouseCursor` false _returnvalue)
  (`WidgetBlueprintLibrary.SetInputMode_GameOnly` _returnvalue)
  (bind _outactors (`GameplayStatics.GetAllActorsOfClass` "/Game/Dynamic/Blueprints/Spawners/BP_FireflySpawner.BP_FireflySpawner_C"))
  (set `self.FireflySpawners` _outactors)
  (`self.SetupFireflySpawns`))

(event `RespawnPlayer`
  (`self.SpawnPlayer`))

(event `self.ReceiveTick`
  (params (DeltaSeconds :type "Float (single-precision)"))
  (set `self.SurvivalTime` (+ DeltaSeconds (`self.SurvivalTime`))))

(event `PlayerDeath`
  (bind _returnvalue (`GameplayStatics.GetPlayerController` 0))
  (`GameplayStatics.SetGamePaused` true)
  (`WidgetLayoutLibrary.RemoveAllWidgets`)
  (bind _returnvalue_2 (`|CreateWidget` "/Game/Dynamic/Blueprints/HUD/BPW_EndScreen.BPW_EndScreen_C"))
  (`UserWidget.AddToViewport` _returnvalue_2 0)
  (set `PlayerController.bShowMouseCursor` true _returnvalue)
  (`WidgetBlueprintLibrary.SetInputMode_UIOnlyEx` _returnvalue _returnvalue_2))

(fn `FlyConsumed`
  (`/Engine/EditorBlueprintResources/StandardMacros.IncrementInt` (`self.FliesConsumed`)))

(fn `FlyDied`
  (`/Engine/EditorBlueprintResources/StandardMacros.IncrementInt` (`self.FliesDied`)))

(fn `SetupFireflySpawns`
  (locals (ChosenSpawnIdx :type Integer :default -1) (FireflySpawner :type "/Game/Dynamic/Blueprints/Spawners/BP_FireflySpawner Object Reference"))
  (for _array_element (`self.FireflySpawners`)
    (`KismetSystemLibrary.K2_SetTimer` _array_element "Spawn" (`KismetMathLibrary.RandomFloatInRange` (`self.MinSpawnTime`) (`self.MaxSpawnTime`)) true)
    (`/Game/Dynamic/Blueprints/Spawners/BP_FireflySpawner.Spawn` _array_element)))

(fn `SpawnPlayer`
  (locals (Food :type "Float (double-precision)"))
  (bind _returnvalue (`GameplayStatics.GetPlayerPawn` 0))
  (bind _returnvalue_2 (`GameplayStatics.GetPlayerController` 0))
  ;[1 1 1] Cleanup old pawn in case not destroyed
  (`/Engine/EditorBlueprintResources/StandardMacros.IsValid` _returnvalue
    (:`Is Valid`
      (bind _asbp_base_spider (cast `/Game/Dynamic/Blueprints/Pawns/Player/BP_BaseSpider` _returnvalue))
      (set `local.Food` (`/Game/Dynamic/Blueprints/Pawns/Player/Components/BPC_Hunger.Food` (`/Game/Dynamic/Blueprints/Pawns/Player/BP_BaseSpider.Hunger` _asbp_base_spider)))
      (`self.K2_DestroyActor` _asbp_base_spider))
    (:`Is Not Valid`
      _))
  ;[1 1 1] Respawn
  (bind _returnvalue_3 (`|SpawnActorFromClass` (`self.DefaultPawnClass`) (`self.GetTransform` (`self.K2_FindPlayerStart` _returnvalue_2)) "Undefined" "MultiplyWithRoot" null null))
  (`Controller.Possess` _returnvalue_2 _returnvalue_3)
  ;[1 1 1] Set food to old food
  (bind _asbp_base_spider_2 (cast `/Game/Dynamic/Blueprints/Pawns/Player/BP_BaseSpider` _returnvalue_3))
  (set `/Game/Dynamic/Blueprints/Pawns/Player/Components/BPC_Hunger.Food` (`local.Food`) (`/Game/Dynamic/Blueprints/Pawns/Player/BP_BaseSpider.Hunger` _asbp_base_spider_2)))

(fn `UserConstructionScript`)